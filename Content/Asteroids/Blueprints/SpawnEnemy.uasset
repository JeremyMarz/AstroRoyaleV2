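; SpawnEnemy is a spawner for an Asteroids game that repeatedly creates asteroid enemies at its own transform.
; On BeginPlay it starts a looping timer that calls the function named in its FunctionName variable every LoopTime seconds.
; SpawnFunctionN and SpawnFunctionNE spawn AsteroidEnemyN and AsteroidEnemyNE respectively, so the name variable selects the enemy variant.
; Debug prints show the chosen function name and each spawn call.
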(event `self.ReceiveTick`
  (params (DeltaSeconds :type "Float (single-precision)")))

(event `self.ReceiveBeginPlay`
  (bind _functionname (`self.functionName`))
  (`KismetSystemLibrary.PrintString` _functionname)
  (`KismetSystemLibrary.K2_SetTimer` null _functionname (`self.LoopTime`) true))

(fn `SpawnFunctionN`
  (`KismetSystemLibrary.PrintString` "Hello")
  (`|SpawnActorFromClass` "/Game/Asteroids/Blueprints/AsteroidEnemyN.AsteroidEnemyN_C" (`self.GetTransform` self) "Undefined" "OverrideRootScale" null null))

(fn `SpawnFunctionNE`
  (`KismetSystemLibrary.PrintString` "Hello")
  (`|SpawnActorFromClass` "/Game/Asteroids/Blueprints/AsteroidEnemyNE.AsteroidEnemyNE_C" (`self.GetTransform` self) "Undefined" "OverrideRootScale" null null))

(fn `UserConstructionScript`)