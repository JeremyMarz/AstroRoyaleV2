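; Medium asteroid enemy that drifts in a random direction and breaks into small asteroids when hit by a ball.
; BeginPlay scales it up and picks random signed X/Y steps sharing a fixed total, then a delay-driven loop teleports it along without sweep.
; A hit from a "Ball"-tagged actor sets flags that end the loop, spawning AsteroidEnemy_Small actors before destruction.
; Reaching MaxMovements without a hit destroys it without splitting.
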(event `self.ReceiveBeginPlay`
  (bind _currentmovement (`self.CurrentMovement`))
  ;[1 1 1] Asteroid Movement
  (bind _output_get (set `self.tempXFloat` (`KismetMathLibrary.RandomFloatInRange` 0.0 20.0)))
  (set `self.tempYFloat` (- 20.0 _output_get))
  (if (not (`KismetMathLibrary.RandomBool`))
    (set `self.tempXFloat` (* -1 (`self.tempXFloat`))))
  (if (not (`KismetMathLibrary.RandomBool`))
    (set `self.tempYFloat` (* -1 (`self.tempYFloat`))))
  (`self.SetActorScale3D` (5.0 5.0 5.0))
  (`self.K2_SetActorLocation` (+ (`self.K2_GetActorLocation`) (`KismetMathLibrary.MakeVector` (`self.tempXFloat`) (`self.tempYFloat`))) :!label _label)
  (if (not (`self.BallDestroy`))
    (`KismetSystemLibrary.Delay` 0.02)
    (if (not (== (`self.MaxMovements`) _currentmovement))
      (bind _result (`/Engine/EditorBlueprintResources/StandardMacros.IncrementInt` _currentmovement)
        (:`  `
          (set `self.CurrentMovement` _result)
          (goto _label)))
      (else
        _)))
  (if (`self.BallHit`)
    (for _ (range (+ (`KismetMathLibrary.RandomIntegerInRange` 1 2) 1))
      (`|SpawnActorFromClass` "/Game/Asteroids/Blueprints/AsteroidEnemy_Small.AsteroidEnemy_Small_C" (`self.GetTransform` self) "Undefined" "OverrideRootScale" null null)))
  (`self.K2_DestroyActor`))

(event `self.ReceiveHit`
  (params (MyComp :type "PrimitiveComponent Object Reference") (Other :type "Actor Object Reference") (OtherComp :type "PrimitiveComponent Object Reference") (bSelfMoved :type Boolean) (HitLocation :type "Vector Structure") (HitNormal :type "Vector Structure") (NormalImpulse :type "Vector Structure") (Hit :type "HitResult Structure (by ref)"))
  (if (`self.ActorHasTag` Other (`KismetStringLibrary.Conv_StringToName` "Ball"))
    (set `self.BallHit` true)
    (set `self.BallDestroy` true)))

(fn `UserConstructionScript`)