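; AsteroidEnemyN is an asteroid enemy actor that drifts along world +X until a ball hits it or it runs out of moves.
; BeginPlay enlarges it, then runs a looped Delay that teleport-steps its location without sweep and counts moves up to MaxMovements.
; Hits from actors tagged "Ball" only set BallDestroy, which the loop checks after each step to destroy the actor.
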(event `self.ReceiveBeginPlay`
  (bind _currentmovement (`self.CurrentMovement`))
  ;[1 1 1] Asteroid Movement
  (`self.SetActorScale3D` (10.0 10.0 10.0))
  (`self.K2_SetActorLocation` (+ (`self.K2_GetActorLocation`) (20.0 0.0 0.0)) :!label _label)
  (if (not (`self.BallDestroy`))
    (`KismetSystemLibrary.Delay` 0.02)
    (if (not (== (`self.MaxMovements`) _currentmovement))
      (bind _result (`/Engine/EditorBlueprintResources/StandardMacros.IncrementInt` _currentmovement)
        (:`  `
          (set `self.CurrentMovement` _result)
          (goto _label)))
      (else
        _)))
  (`self.K2_DestroyActor`))

(event `self.ReceiveHit`
  (params (MyComp :type "PrimitiveComponent Object Reference") (Other :type "Actor Object Reference") (OtherComp :type "PrimitiveComponent Object Reference") (bSelfMoved :type Boolean) (HitLocation :type "Vector Structure") (HitNormal :type "Vector Structure") (NormalImpulse :type "Vector Structure") (Hit :type "HitResult Structure (by ref)"))
  (if (`self.ActorHasTag` Other (`KismetStringLibrary.Conv_StringToName` "Ball"))
    (set `self.BallDestroy` true)))

(fn `UserConstructionScript`)