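; Asteroid Blueprint with random mesh and material pickers, rotating and projectile movement components, and a death drop.
; Randomised spin, planar direction and appearance calls sit in the Construction Script, disconnected from its entry, so they never run.
; ChanceToSpawnCollectible destroys the asteroid, with roughly a one-in-ten chance of spawning BP_Collectible from DeathLocation.
; The event graph is empty, and nothing here calls that drop function.
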(fn `ChanceToSpawnCollectible`
  ;[1 1 1] Chance to drop 'Collectible'
  (if (<= (`KismetMathLibrary.RandomInteger` 101) 10)
    (`|SpawnActorFromClass` "/Game/Blueprints/BP_Collectible.BP_Collectible_C" (`KismetMathLibrary.Conv_VectorToTransform` (`self.deathLocation`)) "Undefined" "OverrideRootScale" null null)
    (`self.K2_DestroyActor`)
    (else
      (`self.K2_DestroyActor`))))

(fn `SelectAsteroidMaterial`
  (bind _asteroid (`self.Asteroid`))
  (switch `int` (`KismetMathLibrary.RandomInteger` 3)
    (:`0`
      (`PrimitiveComponent.SetMaterial` _asteroid 0 "/Game/Asteroids/Materials/M_AsteroidGrey.M_AsteroidGrey"))
    (:`1`
      (`PrimitiveComponent.SetMaterial` _asteroid 0 "/Game/Asteroids/Materials/M_AsteroidBrown.M_AsteroidBrown"))
    (:`2`
      (`PrimitiveComponent.SetMaterial` _asteroid 0 "/Game/Asteroids/Materials/M_AsteroidBlack.M_AsteroidBlack"))))

(fn `SelectStaticMesh`
  (bind _asteroid (`self.Asteroid`))
  (switch `int` (`KismetMathLibrary.RandomInteger` 3)
    (:`0`
      (`StaticMeshComponent.SetStaticMesh` _asteroid "/Game/Assets/Asteroid_01.Asteroid_01"))
    (:`1`
      (`StaticMeshComponent.SetStaticMesh` _asteroid "/Game/Assets/Asteroid_04.Asteroid_04"))
    (:`2`
      (`StaticMeshComponent.SetStaticMesh` _asteroid "/Game/Assets/Asteroid_05.Asteroid_05"))))

(fn `UserConstructionScript`
  ;[1 1 1] Set random roll and velocity, Select one of three meshes and materials at random
)