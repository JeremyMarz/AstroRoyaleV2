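; BP_Collectible is a coin pickup that the player's TwinStickPawn collects by overlapping it.
; On overlap it increments the Collectibles count on BP_PlayerController and destroys itself.
; It then raises the controller's ShotsToFire by one if that value is below one fifth of the collected total, rounded down, tying shot count to coins gathered.
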(event `self.ReceiveActorBeginOverlap`
  (params (OtherActor :type "Actor Object Reference"))
  ;[1 1 1] Collects coin, destroy coin & increment collectibles
  (bind _asbp_player_controller (cast `/Game/TwinStickBP/Blueprints/BP_PlayerController` (`GameplayStatics.GetPlayerController` 0)))
  (cast `/Game/TwinStickBP/Blueprints/TwinStickPawn` OtherActor)
  (bind _collectibles (`/Game/TwinStickBP/Blueprints/BP_PlayerController.Collectibles` _asbp_player_controller))
  (`/Engine/EditorBlueprintResources/StandardMacros.IncrementInt` _collectibles
    (:`  `
      (`self.K2_DestroyActor`)
      (bind _shotstofire (`/Game/TwinStickBP/Blueprints/BP_PlayerController.ShotsToFire` _asbp_player_controller))
      (if (< _shotstofire (`KismetMathLibrary.FFloor` (/ (`KismetMathLibrary.Conv_IntToDouble` _collectibles) 5.0)))
        (`/Engine/EditorBlueprintResources/StandardMacros.IncrementInt` _shotstofire)))))

(fn `UserConstructionScript`)